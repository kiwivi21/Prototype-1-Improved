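; BP_Grapple is a grappling hook gun that pulls the first-person player toward whatever surface they fire at.
; FireGrapple line-traces forward from the player camera, attaches the Hook to the hit actor, shows the Cable, then makes the player jump into Falling movement.
; While attached, Tick adds velocity along the gun-to-hook direction scaled by PullStrength each frame, until ReleaseGrapple detaches the pull and hides the cable.
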(event `self.ReceiveBeginPlay`
  ;[0 0 1] Set player ref
  (bind _asbp_first_person_character (cast `/Game/FirstPerson/Blueprints/BP_FirstPersonCharacter` (`GameplayStatics.GetPlayerCharacter` 0)))
  (set `self.PlayerRef` _asbp_first_person_character))

(event `FireGrapple`
  ;[0 0 1] Fire grapple
  (`self.PlayerRef`
    (:`then`
      _)
    (:`else`
      (bind _asbp_first_person_character (cast `/Game/FirstPerson/Blueprints/BP_FirstPersonCharacter` (`GameplayStatics.GetPlayerCharacter` 0)))
      (set `self.PlayerRef` _asbp_first_person_character)))
  (bind (_returnvalue _hitresult) (`self.CheckForCollision`))
  (if _returnvalue
    (bind (_bblockinghit _binitialoverlap _time _distance _location _impactpoint _normal _impactnormal _physmat _hitactor) (`GameplayStatics.BreakHitResult` _hitresult))
    (set `self.HitLocation` _location)
    (set `self.HitActor` _hitactor)
    (`SceneComponent.K2_SetWorldLocation` (`self.Hook`) (`self.HitLocation`) false false)
    (`SceneComponent.K2_AttachToComponent` (`self.Hook`) (`Actor.RootComponent` (`self.HitActor`)) "None" "KeepWorld" "KeepWorld" "KeepWorld" true)
    (`SceneComponent.SetVisibility` (`self.Cable`) true false)
    (set `self.GrappleAttached` true)
    (`Character.Jump` (`self.PlayerRef`))
    (`CharacterMovementComponent.SetMovementMode` (`Character.CharacterMovement` (`self.PlayerRef`)) "MOVE_Falling" 0)))

(event `ReleaseGrapple`
  ;[0 0 1] Release the grapple
  (set `self.GrappleAttached` false)
  (`SceneComponent.SetVisibility` (`self.Cable`) false false)
  (`CharacterMovementComponent.SetMovementMode` (`Character.CharacterMovement` (`self.PlayerRef`)) "MOVE_Falling" 0))

(event `self.ReceiveTick`
  (params (DeltaSeconds :type "Float (single-precision)"))
  ;[0 0 1] Pull player
  (if (`self.GrappleAttached`)
    (set `MovementComponent.Velocity` (+ (`self.GetVelocity` (`self.PlayerRef`)) (* (`KismetMathLibrary.GetDirectionUnitVector` (`SceneComponent.K2_GetComponentLocation` (`self.Gun`)) (`SceneComponent.K2_GetComponentLocation` (`self.Hook`))) (`self.PullStrength`))) (`Character.CharacterMovement` (`self.PlayerRef`)))))

(fn `CheckForCollision`
  (returns (ReturnValue :type Boolean) (HitResult :type "HitResult Structure"))
  (bind _firstpersoncamera (`/Game/FirstPerson/Blueprints/BP_FirstPersonCharacter.FirstPersonCamera` (`self.PlayerRef`)))
  (bind _returnvalue (`SceneComponent.K2_GetComponentLocation` _firstpersoncamera))
  (bind _returnvalue_2 (`SceneComponent.GetForwardVector` _firstpersoncamera))
  (bind (_outhit _returnvalue_3) (`KismetSystemLibrary.LineTraceSingle` (+ _returnvalue (* _returnvalue_2 50.0)) (+ _returnvalue (* _returnvalue_2 4000.0)) "TraceTypeQuery1"))
  (return _returnvalue_3 _outhit))

(fn `UserConstructionScript`)